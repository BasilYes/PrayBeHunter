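; BP_GrenadeExplosion is the short-lived explosion effect actor for the grenade skill.
; On BeginPlay it scales the PExplosion component uniformly from its Energy value up to a cap, plays an explosion sound at its location, and destroys itself after a short delay.
; It applies no damage itself; an unconnected debug sphere draw, also sized by capped Energy, remains in the graph.
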(event `self.ReceiveBeginPlay`
  (bind _returnvalue (`KismetMathLibrary.FMin` (* (`self.Energy`) 0.25) 25.0))
  (`SceneComponent.SetWorldScale3D` (`self.P_Explosion`) (`KismetMathLibrary.MakeVector` _returnvalue _returnvalue _returnvalue))
  (`GameplayStatics.PlaySoundAtLocation` "/Game/Blueprints/Sounds/Explosion01.Explosion01" (`self.K2_GetActorLocation`) (struct) 1.0 1.0 0.0 null null null) ; Play firing sound
  (`KismetSystemLibrary.Delay` 5.0)
  (`self.K2_DestroyActor`))

(fn `UserConstructionScript`)
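; BP_DefautBullet is a skill projectile that deals Energy-scaled point damage and destroys itself on contact.
; Collision component overlaps affect only player characters other than its owner, with a flat bonus added to the scaled damage.
; The Hit event damages whatever it strikes, without that bonus or an owner check.
; Only the server applies damage, credited to the instigator's controller, while the destroy call has no server check.
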(event `self.CollisionComponent.OnComponentBeginOverlap`
  (params (OverlappedComponent :type "PrimitiveComponent Object Reference") (OtherActor :type "Actor Object Reference") (OtherComp :type "PrimitiveComponent Object Reference") (OtherBodyIndex :type Integer) (bFromSweep :type Boolean) (SweepResult :type "HitResult Structure (by ref)"))
  (bind _returnvalue (`self.GetOwner`))
  (bind _asbp_player_character (cast `/Game/Blueprints/Character/BP_PlayerCharacter` OtherActor))
  (if (!= _asbp_player_character (`self.GetOwner`))
    (if (`KismetSystemLibrary.IsServer`)
      (`GameplayStatics.ApplyPointDamage` _asbp_player_character (+ (* (`self.Energy`) 3.8) 5.0) (`self.K2_GetActorLocation`) SweepResult (`self.GetInstigatorController`) (select `bool` (`KismetSystemLibrary.IsValid` _returnvalue) :`true` _returnvalue)))
    (`self.K2_DestroyActor`)))

(event `self.ReceiveHit`
  (params (MyComp :type "PrimitiveComponent Object Reference") (Other :type "Actor Object Reference") (OtherComp :type "PrimitiveComponent Object Reference") (bSelfMoved :type Boolean) (HitLocation :type "Vector Structure") (HitNormal :type "Vector Structure") (NormalImpulse :type "Vector Structure") (Hit :type "HitResult Structure (by ref)"))
  (bind _returnvalue (`self.GetOwner`))
  (bind _returnvalue_2 (select `bool` (`KismetSystemLibrary.IsValid` _returnvalue) :`true` _returnvalue))
  (if (`KismetSystemLibrary.IsServer`)
    (`GameplayStatics.ApplyPointDamage` Other (* (`self.Energy`) 4.0) (`self.K2_GetActorLocation` _returnvalue_2) Hit (`self.GetInstigatorController`) _returnvalue_2))
  (`self.K2_DestroyActor`))

(event `self.ReceiveBeginPlay`)

(fn `UserConstructionScript`)
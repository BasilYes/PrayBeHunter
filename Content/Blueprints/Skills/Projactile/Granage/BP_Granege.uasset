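; Grenade projectile actor that explodes on its first hit or after a short fuse, whichever comes first.
; A DoOnce guards the detonation, which applies full radial damage with strength and capped radius scaled by its Energy value.
; The explosion event then spawns BP_GranageExplosion with that Energy everywhere except dedicated servers, and destroys the grenade.
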(event `self.ReceiveBeginPlay`
  (bind _energy (`self.Energy`))
  (`KismetSystemLibrary.Delay` 2.0)
  (`/Engine/EditorBlueprintResources/StandardMacros.DoOnce` false :!label _label
    (:`Completed`
      (`GameplayStatics.ApplyRadialDamage` :`BaseDamage` (* _energy 3.0) :`Origin` (`self.K2_GetActorLocation`) :`DamageRadius` (`KismetMathLibrary.FMin` (* _energy 10.0) 1000.0) :`DamageCauser` self :`InstigatedByController` (`self.GetInstigatorController`) :`bDoFullDamage` true :`DamagePreventionChannel` "ECC_WorldStatic")
      (`self.EventExplosion` (`self.Energy`)))))

(event `self.ReceiveHit`
  (params (MyComp :type "PrimitiveComponent Object Reference") (Other :type "Actor Object Reference") (OtherComp :type "PrimitiveComponent Object Reference") (bSelfMoved :type Boolean) (HitLocation :type "Vector Structure") (HitNormal :type "Vector Structure") (NormalImpulse :type "Vector Structure") (Hit :type "HitResult Structure (by ref)"))
  (goto _label))

(event `EventExplosion`
  (params (Energy :type "Float (double-precision)"))
  (if (not (`KismetSystemLibrary.IsDedicatedServer`))
    (`|SpawnActorFromClass` "/Game/Blueprints/Skills/Projactile/Granage/BP_GranageExplosion.BP_GranageExplosion_C" (`KismetMathLibrary.MakeTransform` (`self.K2_GetActorLocation`)) "AlwaysSpawn" "OverrideRootScale" (`self.GetOwner`) Energy (`self.GetInstigator`)))
  (`self.K2_DestroyActor`))

(fn `UserConstructionScript`
  (`parent.UserConstructionScript`))
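; BP_Trap is a skill trap that drains stamina from player characters other than its owner who step into it.
; It drops its Projectile component on first hit, then a server-side sphere overlap deals radial stamina damage scaled by remaining Energy.
; Triggering plays a collapse sound, spawns a BP_TrapWidget at the victim's location and destroys the trap.
; A server timer decays Energy until the trap expires, and any damage destroys it.
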(event `self.ReceiveHit`
  (params (MyComp :type "PrimitiveComponent Object Reference") (Other :type "Actor Object Reference") (OtherComp :type "PrimitiveComponent Object Reference") (bSelfMoved :type Boolean) (HitLocation :type "Vector Structure") (HitNormal :type "Vector Structure") (NormalImpulse :type "Vector Structure") (Hit :type "HitResult Structure (by ref)"))
  (`/Engine/EditorBlueprintResources/StandardMacros.DoOnce` false
    (:`Completed`
      (`ActorComponent.K2_DestroyComponent` (`self.Projectile`)))))

(event `self.ReceiveAnyDamage`
  (params (Damage :type "Float (single-precision)") (DamageType :type "DamageType Object Reference") (InstigatedBy :type "Controller Object Reference") (DamageCauser :type "Actor Object Reference"))
  (`self.K2_DestroyActor`))

(event `EventUse`
  (if (not (`KismetSystemLibrary.IsDedicatedServer`))
    (`GameplayStatics.PlaySoundAtLocation` "/Game/ShowIt/StarterContent/Audio/Collapse_Cue.Collapse_Cue" (`self.K2_GetActorLocation`) (struct) 1.0 1.0 0.0 null null null)))

(event `EventUseOwner`
  (params (Location :type "Vector Structure"))
  (`|SpawnActorFromClass` "/Game/Blueprints/Skills/Trap/BP_TrapWidget.BP_TrapWidget_C" (`KismetMathLibrary.MakeTransform` Location) "AlwaysSpawn" "OverrideRootScale" null (`self.GetInstigator`)))

(event `self.Sphere1.OnComponentBeginOverlap`
  (params (OverlappedComponent :type "PrimitiveComponent Object Reference") (OtherActor :type "Actor Object Reference") (OtherComp :type "PrimitiveComponent Object Reference") (OtherBodyIndex :type Integer) (bFromSweep :type Boolean) (SweepResult :type "HitResult Structure (by ref)"))
  (if (`KismetSystemLibrary.IsServer`)
    (bind _asbp_player_character (cast `/Game/Blueprints/Character/BP_PlayerCharacter` OtherActor))
    (if (!= _asbp_player_character (`self.GetOwner`))
      (`GameplayStatics.ApplyRadialDamage` :`BaseDamage` (* (`self.Energy`) 4.0) :`Origin` (`self.K2_GetActorLocation`) :`DamageRadius` 150.0 :`DamageTypeClass` "/Game/Blueprints/Character/BP_StaminaDamage.BP_StaminaDamage_C" :`DamageCauser` self :`InstigatedByController` (`self.GetInstigatorController`) :`bDoFullDamage` true :`DamagePreventionChannel` "ECC_WorldStatic")
      (`self.EventUse`)
      (`self.EventUseOwner` (`self.K2_GetActorLocation` _asbp_player_character))
      (`self.K2_DestroyActor`))))

(event `self.ReceiveBeginPlay`
  (if (`KismetSystemLibrary.IsServer`)
    (`KismetSystemLibrary.K2_SetTimerDelegate` (delegate `TIck`) 1.0 true)))

(event `TIck`
  (bind _output_get (set `self.Energy` (- (`self.Energy`) 0.5)))
  (if (<= _output_get 0.0)
    (`self.K2_DestroyActor`)))

(fn `UserConstructionScript`
  (`parent.UserConstructionScript`))
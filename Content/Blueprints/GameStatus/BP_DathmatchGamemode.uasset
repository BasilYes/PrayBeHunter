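; Deathmatch game mode that starts the match on BeginPlay through BP_DeathmatchGameStats and handles player deaths.
; PlayerDeath updates kills, deaths and points on BP_PlayerState, rewarding a valid killer and penalizing self-kills more heavily.
; ToSpectrator spawns a spectator pawn at the map's spectator point, copies character, gun and modification types, possesses it and destroys the old character.
; StopMatch is empty.
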(event `self.ReceiveBeginPlay`
  (`self.StartMatch`))

(fn `PlayerDeath`
  (params (Character :type "/Game/Blueprints/Character/BP_PlayerCharacter Object Reference") (Controller :type "/Game/Blueprints/Character/BP_PlayerController Object Reference") (Owner :type "/Game/Blueprints/Character/BP_PlayerController Object Reference"))
  (`self.ToSpectrator` Controller Character)
  (bind _asbp_player_state (cast `/Game/Blueprints/Character/BP_PlayerState` (`Controller.PlayerState` Controller)))
  (set `/Game/Blueprints/Character/BP_PlayerState.Deaths` (+ (`/Game/Blueprints/Character/BP_PlayerState.Deaths` _asbp_player_state) 1) _asbp_player_state)
  (set `/Game/Blueprints/Character/BP_PlayerState.Points` (- (`/Game/Blueprints/Character/BP_PlayerState.Points` _asbp_player_state) 2) _asbp_player_state)
  (if (!= Controller Owner)
    (`/Engine/EditorBlueprintResources/StandardMacros.IsValid` Owner
      (:`Is Valid`
        (bind _asbp_player_state_2 (cast `/Game/Blueprints/Character/BP_PlayerState` (`Controller.PlayerState` Owner)))
        (set `/Game/Blueprints/Character/BP_PlayerState.Kills` (+ (`/Game/Blueprints/Character/BP_PlayerState.Kills` _asbp_player_state_2) 1) _asbp_player_state_2)
        (set `/Game/Blueprints/Character/BP_PlayerState.Points` (+ (`/Game/Blueprints/Character/BP_PlayerState.Points` _asbp_player_state_2) 10) _asbp_player_state_2)))
    (else
      (set `/Game/Blueprints/Character/BP_PlayerState.Points` (- (`/Game/Blueprints/Character/BP_PlayerState.Points` _asbp_player_state) 3) _asbp_player_state))))

(fn `SetMapDefauts`
  (params (SpectratorPoint :type "TargetPoint Object Reference"))
  (set `self.SpectratorPoint` SpectratorPoint))

(fn `StartMatch`
  (bind _asbp_deathmatch_game_stats (cast `/Game/Blueprints/GameStatus/BP_DeathmatchGameStats` (`GameplayStatics.GetGameState`)))
  (`/Game/Blueprints/GameStatus/BP_DeathmatchGameStats.StartMatch` _asbp_deathmatch_game_stats)
  (set `self.MatchStarted` true))

(fn `StopMatch`)

(fn `ToSpectrator`
  (params (Controller :type "Controller Object Reference") (Character :type "/Game/Blueprints/Character/BP_PlayerCharacter Object Reference"))
  (bind _returnvalue (`|SpawnActorFromClass` "/Game/Blueprints/GameStatus/BP_SpectratorPawn.BP_SpectratorPawn_C" (`self.GetTransform` (`self.SpectratorPoint`)) "Undefined" "OverrideRootScale" Controller (`/Game/Blueprints/Character/BP_PlayerCharacter.CharacterType` Character) (`/Game/Blueprints/Character/BP_PlayerCharacter.GunType` Character) (`/Game/Blueprints/Character/BP_PlayerCharacter.ModificationType` Character) Character))
  (`Controller.Possess` Controller _returnvalue)
  (`/Engine/EditorBlueprintResources/StandardMacros.IsValid` Character
    (:`Is Valid`
      (`self.K2_DestroyActor` Character))))

(fn `UserConstructionScript`)
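; Spectator pawn that handles the death and respawn screen in a deathmatch game.
; On possession in a started match, it shows W_DeathMenu with a countdown, plus W_ChoseName while the player still has the placeholder name.
; Once the countdown ends and a name is set, F reads the character, gun and modification selections.
; It spawns that character at a random SpawnPoint, retrying on failure, then possesses it and destroys itself.
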(event `self.ReceiveTick`
  (params (DeltaSeconds :type "Float (single-precision)")))

(event `Key|F`
  (params (Key :type "Key Structure"))
  (bind _menu (`self.Menu`))
  (:`Pressed`
    (bind _asbp_player_state (cast `/Game/Blueprints/Character/BP_PlayerState` (`self.PlayerState`)))
    (if (`KismetTextLibrary.NotEqual_TextText` (`/Game/Blueprints/Character/BP_PlayerState.Name` _asbp_player_state) "Игруньчик")
      (if (< (`self.TimerCounter`) 0)
        (`Widget.RemoveFromParent` (`self.Menu`))
        (bind _asbp_player_controller (cast `/Game/Blueprints/Character/BP_PlayerController` (`self.GetController`)))
        (set `PlayerController.bShowMouseCursor` false _asbp_player_controller)
        (`WidgetBlueprintLibrary.SetInputMode_GameOnly` _asbp_player_controller)
        (`self.EventRespawn` (cast `/Game/Blueprints/Character/E_CharacterType` (`KismetMathLibrary.Conv_IntToByte` (`ComboBoxString.GetSelectedIndex` (`/Game/Blueprints/Widgets/W_DeathMenu.CharacterType` _menu)))) (cast `/Game/Blueprints/Character/GunsComponents/E_GunsComponents` (`KismetMathLibrary.Conv_IntToByte` (`ComboBoxString.GetSelectedIndex` (`/Game/Blueprints/Widgets/W_DeathMenu.GunType` _menu)))) (cast `/Game/Blueprints/Character/GunsModifications/E_GunsModificationsComponents` (`KismetMathLibrary.Conv_IntToByte` (`ComboBoxString.GetSelectedIndex` (`/Game/Blueprints/Widgets/W_DeathMenu.GunModificationType` _menu)))))))))

(event `EventRespawn`
  (params (Character :type "/Game/Blueprints/Character/E_CharacterType Enum" :default "NewEnumerator0") (GunType :type "/Game/Blueprints/Character/GunsComponents/E_GunsComponents Enum" :default "NewEnumerator0") (GunModificationType :type "/Game/Blueprints/Character/GunsModifications/E_GunsModificationsComponents Enum" :default "NewEnumerator0"))
  (if (`self.Yes`)
    (bind _outactors (`GameplayStatics.GetAllActorsOfClass` "/Game/Blueprints/GameStatus/SpawnPoint.SpawnPoint_C"))
    (bind _returnvalue (`|SpawnActorFromClass` (select `/Game/Blueprints/Character/E_CharacterType` Character :`NewEnumerator0` "/Game/Blueprints/Character/Characters/BP_PlayerCharacter_Speed.BP_PlayerCharacter_Speed_C" :`NewEnumerator1` "/Game/Blueprints/Character/Characters/BP_PlayerCharacter_Jump.BP_PlayerCharacter_Jump_C" :!type "/Game/Blueprints/Character/BP_PlayerCharacter Class Reference") (`self.GetTransform` (`|GetArrayItem` _outactors (`KismetMathLibrary.RandomIntegerInRange` 0 (`KismetArrayLibrary.Array_LastIndex` _outactors)))) "Undefined" "OverrideRootScale" self GunType GunModificationType (`self.GetInstigator`) :!label _label))
    (`/Engine/EditorBlueprintResources/StandardMacros.IsValid` _returnvalue
      (:`Is Valid`
        (`Controller.Possess` (`self.GetController`) _returnvalue)
        (`self.K2_DestroyActor`))
      (:`Is Not Valid`
        (goto _label)))))

(event `EventSpawnWidget`
  (params (`Character type` :type "/Game/Blueprints/Character/E_CharacterType Enum" :default "NewEnumerator0") (GunType :type "/Game/Blueprints/Character/GunsComponents/E_GunsComponents Enum" :default "NewEnumerator0") (GunModificationType :type "/Game/Blueprints/Character/GunsModifications/E_GunsModificationsComponents Enum" :default "NewEnumerator0"))
  (bind _playerstate (`self.PlayerState`))
  (set `self.CharacterType` `Character type`)
  (set `self.GunType` GunType)
  (set `self.GunModificationType` GunModificationType)
  (bind _asbp_player_controller (cast `/Game/Blueprints/Character/BP_PlayerController` (`self.GetController`)))
  (`WidgetBlueprintLibrary.SetInputMode_GameAndUIEx` _asbp_player_controller null)
  (set `PlayerController.bShowMouseCursor` true _asbp_player_controller)
  (`/Engine/EditorBlueprintResources/StandardMacros.IsValid` _playerstate :!label _label_2
    (:`Is Valid`
      (`|ExecutionSequence`
        (:`then_0`
          (bind _returnvalue (`KismetSystemLibrary.K2_SetTimerDelegate` (delegate `TimerEvent`) 1.0 true))
          (set `self.Timer` _returnvalue)
          (`|ExecutionSequence`
            (:`then_0`
              (bind _asbp_player_controller_2 (cast `/Game/Blueprints/Character/BP_PlayerController` (`self.GetController`)))
              (bind _returnvalue_2 (`|CreateWidget` "/Game/Blueprints/Widgets/W_DeathMenu.W_DeathMenu_C" _asbp_player_controller_2))
              (bind _output_get (set `self.Menu` _returnvalue_2))
              (`/Game/Blueprints/Widgets/W_DeathMenu.refresh` _output_get (`self.CharacterType`) (`self.GunType`) (`self.GunModificationType`))
              (`UserWidget.AddToViewport` _output_get 0))
            (:`then_1`
              (`TextBlock.SetText` (`/Game/Blueprints/Widgets/W_DeathMenu.Timer` (`self.Menu`)) (`KismetTextLibrary.Conv_IntToText` (`self.TimerCounter`)) :!label _label_3))))
        (:`then_1`
          (bind _asbp_player_state (cast `/Game/Blueprints/Character/BP_PlayerState` _playerstate))
          (if (`KismetTextLibrary.EqualEqual_TextText` (`/Game/Blueprints/Character/BP_PlayerState.Name` _asbp_player_state) "Игруньчик")
            (bind _returnvalue_3 (`|CreateWidget` "/Game/Blueprints/Widgets/W_ChoseName.W_ChoseName_C" (cast `PlayerController` (`self.GetController`) :!pure true) _asbp_player_state))
            (`UserWidget.AddToViewport` _returnvalue_3 0)))))
    (:`Is Not Valid`
      (`KismetSystemLibrary.Delay` 1.0)
      (goto _label_2))))

(event `TimerEvent`
  (bind _output_get (set `self.TimerCounter` (- (`self.TimerCounter`) 1)))
  (if (>= _output_get 0)
    (goto _label_3)
    (else
      (`KismetSystemLibrary.K2_ClearAndInvalidateTimerHandle` (`self.Timer`))
      (`TextBlock.SetText` (`/Game/Blueprints/Widgets/W_DeathMenu.Timer` (`self.Menu`)) "Press \"F\" to respawn!"))))

(event `self.ReceivePossessed`
  (params (NewController :type "Controller Object Reference"))
  (bind _asbp_deathmatch_game_stats (cast `/Game/Blueprints/GameStatus/BP_DeathmatchGameStats` (`GameplayStatics.GetGameState`)))
  (if (`/Game/Blueprints/GameStatus/BP_DeathmatchGameStats.MatchStarted` _asbp_deathmatch_game_stats)
    (`self.EventSpawnWidget` (`self.CharacterType`) (`self.GunType`) (`self.GunModificationType`))
    (`KismetSystemLibrary.Delay` (`KismetMathLibrary.Conv_IntToDouble` (`self.TimerCounter`)))
    (set `self.Yes` true)
    (else
      (`self.NewMatchWidgets`))))

(event `NewMatchWidgets`)

(fn `UserConstructionScript`)
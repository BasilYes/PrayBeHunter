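; Deathmatch game stats Blueprint that tracks elapsed match time and relays kill notifications to the HUD.
; StartMatch resets the match time, starts a looping one-second timer that increments it, and flags the match as started.
; KillEvent skips dedicated servers and posts the victim and killer to the kill chat on the first player controller's HUD widget.
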(event `KillEvent`
  (params (pley :type Text) (Killer :type Text))
  (if (not (`KismetSystemLibrary.IsDedicatedServer`))
    (bind _asbp_player_controller (cast `/Game/Blueprints/Character/BP_PlayerController` (`GameplayStatics.GetPlayerController` 0)))
    (bind _w_hud (`/Game/Blueprints/Character/BP_PlayerController.W_Hud` _asbp_player_controller))
    (`/Engine/EditorBlueprintResources/StandardMacros.IsValid` _w_hud
      (:`Is Valid`
        (`/Game/Blueprints/Widgets/InGameHUD/W_NotCharacterHUd.AddKillChatMessage` _w_hud pley Killer)))))

(fn `MatchTimerTIck`
  (set `self.MatchTime` (+ (`self.MatchTime`) (`KismetMathLibrary.MakeTimespan` 0 0 0 1))))

(fn `StartMatch`
  (set `self.MatchTime` (struct))
  (bind _returnvalue (`KismetSystemLibrary.K2_SetTimer` null "MatchTimerTIck" 1.0 true))
  (set `self.MatchTimer` _returnvalue)
  (set `self.MatchStarted` true))

(fn `UserConstructionScript`)
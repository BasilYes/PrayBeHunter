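; Speed variant of the player character that adds an energy-fuelled sprint held on Shift.
; Sprinting starts only when movement is allowed and Energy suffices, raises walk speed through EventChangeSpeed, and disables CanMove and gun presses.
; While sprinting on the ground, Tick auto-runs along control yaw and overrides movement axes, which work again when falling.
; The server drains Energy during grounded sprint and ends it at zero.
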(event `EventSprint`
  (params (IsSprint :type Boolean))
  (bind _charactermovement (`self.CharacterMovement`))
  (if IsSprint
    (if (and (`self.CanMove`) (>= (`self.Energy`) 5.0))
      (set `self.IsSprint` true)
      (`self.ChangeCanMove` false)
      (bind _output_get (set `CharacterMovementComponent.MaxWalkSpeed` 1500.0 _charactermovement))
      (`self.EventChangeSpeed` _output_get))
    (elif (`self.IsSprint`)
      (set `self.IsSprint` false)
      (`self.ChangeCanMove` true)
      (bind _output_get_2 (set `CharacterMovementComponent.MaxWalkSpeed` 600.0 _charactermovement))
      (`self.EventChangeSpeed` _output_get_2))))

(event `InputAction|Shift`
  (params (Key :type "Key Structure"))
  (:`Pressed`
    (if (and (`self.CanMove`) (>= (`self.Energy`) 5.0))
      (`self.EventSprint` true)))
  (:`Released`
    (`self.EventSprint` false)))

(event `self.ReceiveTick`
  (params (DeltaSeconds :type "Float (single-precision)"))
  (`parent.ReceiveTick` DeltaSeconds)
  (if (and (`self.IsSprint`) (not (`NavMovementComponent.IsFalling` (`self.CharacterMovement`))))
    (`self.AddMovementInput` (`KismetMathLibrary.GetForwardVector` (`KismetMathLibrary.MakeRotator` 0.0 0.0 (.yaw (`self.GetControlRotation`)))))
    (if (`KismetSystemLibrary.IsServer`)
      (bind _output_get (set `self.Energy` (`KismetMathLibrary.FMax` (- (`self.Energy`) (* (`GameplayStatics.GetWorldDeltaSeconds`) 10.0)))))
      (if (<= _output_get 0.0)
        (`self.EventSprint` false)))))

(event `InputAxis|MoveForward` :overrideparent false
  (params (AxisValue :type "Float (single-precision)"))
  (if (not (and (`self.IsSprint`) (not (`NavMovementComponent.IsFalling` (`self.CharacterMovement`)))))
    (`self.AddMovementInput` (`KismetMathLibrary.GetForwardVector` (`KismetMathLibrary.MakeRotator` 0.0 0.0 (.yaw (`self.GetControlRotation`)))) AxisValue)))

(event `InputAxis|MoveRight` :overrideparent false
  (params (AxisValue :type "Float (single-precision)"))
  (if (not (and (`self.IsSprint`) (not (`NavMovementComponent.IsFalling` (`self.CharacterMovement`)))))
    (`self.AddMovementInput` (`KismetMathLibrary.GetRightVector` (`KismetMathLibrary.MakeRotator` 0.0 0.0 (.yaw (`self.GetControlRotation`)))) AxisValue)))

(event `self.EventGunPressed`
  (params (Pressed :type Boolean))
  (if (not (`self.IsSprint`))
    (`parent.EventGunPressed` Pressed)))

(fn `UserConstructionScript`
  (`parent.UserConstructionScript`))
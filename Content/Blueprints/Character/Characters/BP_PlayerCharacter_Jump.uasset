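; Player character Blueprint that adds an energy-powered high jump.
; Holding Shift with enough Energy arms the boost by raising the movement component's JumpZVelocity, and releasing it restores the lower value.
; Pressing Jump while boosted deducts JumpCost if the character can move and is grounded, otherwise cancels the boost, then calls the regular Jump either way.
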(event `EventJump`
  (params (IsJump :type Boolean))
  (if IsJump
    (if (>= (`self.Energy`) (`self.JumpCost`))
      (set `self.Shift` true)
      (set `CharacterMovementComponent.JumpZVelocity` 1000.0 (`self.CharacterMovement`)))
    (else
      (set `self.Shift` false)
      (set `CharacterMovementComponent.JumpZVelocity` 500.0 (`self.CharacterMovement`)))))

(event `InputAction|Shift`
  (params (Key :type "Key Structure"))
  (:`Pressed`
    (if (and (`self.CanMove`) (>= (`self.Energy`) (`self.JumpCost`)))
      (`self.EventJump` true)))
  (:`Released`
    (`self.EventJump` false)))

(event `EventExtraJump`
  (if (`self.Shift`)
    (if (and (`self.CanMove`) (>= (`self.Energy`) (`self.JumpCost`)) (not (`NavMovementComponent.IsFalling` (`self.CharacterMovement`))))
      (set `self.Energy` (- (`self.Energy`) (`self.JumpCost`)))
      (else
        (`self.EventJump` false)))))

(event `self.ReceiveTick`
  (params (DeltaSeconds :type "Float (single-precision)"))
  (`parent.ReceiveTick` DeltaSeconds))

(event `InputAction|Jump`
  (params (Key :type "Key Structure"))
  (:`Pressed`
    (`self.EventExtraJump`)
    (`self.Jump`)))

(fn `UserConstructionScript`
  (`parent.UserConstructionScript`))
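; Gun component that gives BP_PlayerCharacter a default projectile shot, allowed while EnergyInGun is at least 1.
; Fire line-traces on the Camera channel from the camera, combining actor yaw and roll with the character's aim pitch.
; It plays the shot sound and spawns the projectile class at the FPGun muzzle, rotated toward the hit point or trace end to converge on the aim.
; The projectile receives the gun's energy, with the character as owner and instigator.
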(fn `CanFire`
  (returns (Can :type Boolean))
  (bind _asbp_player_character (cast `/Game/Blueprints/Character/BP_PlayerCharacter` (`self.GetOwner`)))
  (return (>= (`/Game/Blueprints/Character/BP_PlayerCharacter.EnergyInGun` _asbp_player_character) 1.0)))

(fn `Fire`
  (returns (Fired :type Boolean))
  (bind _asbp_player_character (cast `/Game/Blueprints/Character/BP_PlayerCharacter` (`self.GetOwner`)))
  (bind _returnvalue (`SceneComponent.K2_GetComponentLocation` (`/Game/Blueprints/Character/BP_PlayerCharacter.Camera` _asbp_player_character)))
  (bind (_returnvalue_roll _returnvalue_pitch _returnvalue_yaw) (`KismetMathLibrary.BreakRotator` (`Actor.K2_GetActorRotation` _asbp_player_character)))
  (bind _outhit (`KismetSystemLibrary.LineTraceSingle` _returnvalue (+ (* (`KismetMathLibrary.Conv_RotatorToVector` (`KismetMathLibrary.MakeRotator` _returnvalue_roll (`/Game/Blueprints/Character/BP_PlayerCharacter.AimDerection` _asbp_player_character) _returnvalue_yaw)) 5000) _returnvalue) "TraceTypeQuery2"))
  (bind _returnvalue_2 (`SceneComponent.GetSocketLocation` (`/Game/Blueprints/Character/BP_PlayerCharacter.FP_Gun` _asbp_player_character) "Muzzle"))
  (`/Game/Blueprints/Character/BP_PlayerCharacter.PlaySound` _asbp_player_character _returnvalue_2)
  (bind (_bblockinghit _binitialoverlap _time _distance _location _impactpoint _normal _impactnormal _physmat _hitactor _hitcomponent _hitbonename _hititem _faceindex _tracestart _traceend) (`GameplayStatics.BreakHitResult` _outhit))
  (`|SpawnActorFromClass` (`self.ProjatileClass`) (`KismetMathLibrary.MakeTransform` _returnvalue_2 (`KismetMathLibrary.Conv_VectorToRotator` (- (select `bool` _bblockinghit :`false` _traceend :`true` _location) _returnvalue_2))) "AlwaysSpawn" "OverrideRootScale" _asbp_player_character (`/Game/Blueprints/Character/BP_PlayerCharacter.EnergyInGun` _asbp_player_character) _asbp_player_character)
  (`self.Value`)
  (return true))
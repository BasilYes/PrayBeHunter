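; Sniper gun component for BP_PlayerCharacter that fires a hitscan shot powered by the energy in the gun, allowed above a minimum charge.
; Fire traces from the camera along the aim, then from the supplied Target origin toward that point to find the actual hit.
; The shot deals point damage and sends a rotation add to the player controller, both scaled by energy.
; It also plays an explosion sound and draws a debug line.
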(event `EventTrace`
  (params (Start :type "Vector Structure") (End :type "Vector Structure"))
  (`KismetSystemLibrary.DrawDebugLine` Start End (struct :`R` 1.0 :`A` 1.0) 2.5 2.0))

(fn `CanFire`
  (returns (Can :type Boolean))
  (bind _asbp_player_character (cast `/Game/Blueprints/Character/BP_PlayerCharacter` (`self.GetOwner`)))
  (return (>= (`/Game/Blueprints/Character/BP_PlayerCharacter.EnergyInGun` _asbp_player_character) 10.0)))

(fn `Fire`
  (params (Target :type "Vector Structure"))
  (returns (Fired :type Boolean))
  (bind _asbp_player_character (cast `/Game/Blueprints/Character/BP_PlayerCharacter` (`self.GetOwner`)))
  (bind _returnvalue (`SceneComponent.K2_GetComponentLocation` (`/Game/Blueprints/Character/BP_PlayerCharacter.Camera` _asbp_player_character)))
  (bind (_returnvalue_roll _returnvalue_pitch _returnvalue_yaw) (`KismetMathLibrary.BreakRotator` (`Actor.K2_GetActorRotation` _asbp_player_character)))
  (bind _outhit (`KismetSystemLibrary.LineTraceSingle` _returnvalue (+ (* (`KismetMathLibrary.Conv_RotatorToVector` (`KismetMathLibrary.MakeRotator` _returnvalue_roll (`/Game/Blueprints/Character/BP_PlayerCharacter.AimDerection` _asbp_player_character) _returnvalue_yaw)) 10000) _returnvalue) "TraceTypeQuery2"))
  (bind (_bblockinghit _binitialoverlap _time _distance _location _impactpoint _normal _impactnormal _physmat _hitactor _hitcomponent _hitbonename _hititem _faceindex _tracestart _traceend) (`GameplayStatics.BreakHitResult` _outhit))
  (bind _outhit_2 (`KismetSystemLibrary.LineTraceSingle` Target (select `bool` _bblockinghit :`false` _traceend :`true` _location) "TraceTypeQuery2"))
  (bind (_bblockinghit_2 _binitialoverlap_2 _time_2 _distance_2 _location_2 _impactpoint_2 _normal_2 _impactnormal_2 _physmat_2 _hitactor_2 _hitcomponent_2 _hitbonename_2 _hititem_2 _faceindex_2 _tracestart_2 _traceend_2) (`GameplayStatics.BreakHitResult` _outhit_2))
  (bind _returnvalue_2 (select `bool` _bblockinghit_2 :`false` _traceend_2 :`true` _location_2))
  (`self.EventTrace` Target _returnvalue_2)
  (`/Game/Blueprints/Character/BP_PlayerCharacter.PlaySound` _asbp_player_character "/Game/ShowIt/StarterContent/Audio/Explosion_Cue.Explosion_Cue" Target)
  (bind _energyingun (`/Game/Blueprints/Character/BP_PlayerCharacter.EnergyInGun` _asbp_player_character))
  (bind _returnvalue_3 (`Pawn.GetController` _asbp_player_character))
  (`GameplayStatics.ApplyPointDamage` _hitactor_2 (* _energyingun 2.5) _returnvalue_2 _outhit_2 _returnvalue_3 _returnvalue_3)
  (bind _asbp_player_controller (cast `/Game/Blueprints/Character/BP_PlayerController` (`Pawn.GetController` _asbp_player_character)))
  (`/Game/Blueprints/Character/BP_PlayerController.Event add rotator` _asbp_player_controller (* _energyingun 0.25))
  (`self.Value`)
  (return true))
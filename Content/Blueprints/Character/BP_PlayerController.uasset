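; Player controller that manages local HUD widgets and feeds aim pitch to BP_PlayerCharacter.
; BeginPlay creates the scoreboard, fast menu and non-character HUD only for local players; holding Tab shows refreshed stats, while Escape or Delete closes the fast menu.
; Possess shows bars and target widgets for player characters and hides them otherwise, via EventRemoveWidgets, whose Remove=true actually adds them.
; Tick copies controller pitch into AimDerection; addrotator offsets control pitch.
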(event `Event add rotator`
  (params (Rotator :type "Float (double-precision)"))
  (`self.SetControlRotation` (`KismetMathLibrary.MakeRotator` (.roll (`self.GetControlRotation`)) (+ (.pitch (`self.GetControlRotation`)) Rotator) (.yaw (`self.GetControlRotation`)))))

(event `self.ReceiveTick`
  (params (DeltaSeconds :type "Float (single-precision)"))
  (bind (_returnvalue_roll _returnvalue_pitch) (`KismetMathLibrary.BreakRotator` (`self.K2_GetActorRotation`)))
  (bind _asbp_player_character (cast `/Game/Blueprints/Character/BP_PlayerCharacter` (`self.K2_GetPawn`)))
  (set `/Game/Blueprints/Character/BP_PlayerCharacter.AimDerection` _returnvalue_pitch _asbp_player_character))

(event `self.ReceivePossess`
  (params (PossessedPawn :type "Pawn Object Reference"))
  (cast `/Game/Blueprints/Character/BP_PlayerCharacter` PossessedPawn
    (:`then`
      (`self.EventRemoveWidgets` true))
    (:`CastFailed`
      (`self.EventRemoveWidgets` false))))

(event `EventRemoveWidgets`
  (params (Remove :type Boolean))
  (if Remove
    (`/Engine/EditorBlueprintResources/StandardMacros.IsValid` (`self.W_Bars`)
      (:`Is Valid`
        _)
      (:`Is Not Valid`
        (bind _returnvalue (`|CreateWidget` "/Game/Blueprints/Widgets/InGameHUD/W_Bars.W_Bars_C" self))
        (set `self.W_Bars` _returnvalue)
        (bind _returnvalue_2 (`|CreateWidget` "/Game/Blueprints/Widgets/InGameHUD/W_Target.W_Target_C" self))
        (set `self.W_Traget` _returnvalue_2)))
    (`UserWidget.AddToViewport` (`self.W_Bars`) 0)
    (`UserWidget.AddToViewport` (`self.W_Traget`) 0)
    (else
      (`/Engine/EditorBlueprintResources/StandardMacros.IsValid` (`self.W_Bars`)
        (:`Is Valid`
          (`Widget.RemoveFromParent` (`self.W_Bars`))
          (`Widget.RemoveFromParent` (`self.W_Traget`)))))))

(event `self.ReceiveBeginPlay`
  (if (`KismetSystemLibrary.IsDedicatedServer`)
    _
    (elif (`KismetSystemLibrary.IsServer`)
      (if (== (`GameplayStatics.GetPlayerController` 0) self)
        (bind _returnvalue (`|CreateWidget` "/Game/Blueprints/Widgets/W_Tab.W_Tab_C" self :!label _label))
        (set `self.TabMenu` _returnvalue)
        (bind _returnvalue_2 (`|CreateWidget` "/Game/Blueprints/Widgets/W_FastMenu.W_FastMenu_C" self))
        (set `self.W_Menu` _returnvalue_2)
        (bind _returnvalue_3 (`|CreateWidget` "/Game/Blueprints/Widgets/InGameHUD/W_NotCharacterHUd.W_NotCharacterHUd_C" self))
        (bind _output_get (set `self.W_Hud` _returnvalue_3))
        (`UserWidget.AddToViewport` _output_get 0))
      (else
        (goto _label)))))

(event `Key|Escape`
  (params (Key :type "Key Structure"))
  (:`Pressed`
    (`/Game/Blueprints/Widgets/W_FastMenu.remove from parent` (`self.W_Menu`) :!label _label_2)))

(event `Key|Delete`
  (params (Key :type "Key Structure"))
  (:`Pressed`
    (goto _label_2)))

(event `Key|Tab`
  (params (Key :type "Key Structure"))
  (bind _tabmenu (`self.TabMenu`))
  (:`Pressed`
    (`UserWidget.AddToViewport` _tabmenu 0)
    (`/Game/Blueprints/Widgets/W_Tab.refreshPlayerStats` _tabmenu))
  (:`Released`
    (`Widget.RemoveFromParent` _tabmenu)))

(fn `UserConstructionScript`)
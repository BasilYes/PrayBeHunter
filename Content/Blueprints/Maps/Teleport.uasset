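; Teleporter map actor that moves any actor overlapping its capsule to a randomly chosen linked teleporter from its Duo array.
; The server performs the teleport while usable, preserving the actor's offset from the pad.
; ChangeUsable runs on both source and destination pads, starting a ten-second cooldown that prevents immediate bounce-back.
; Its spark effect hides during cooldown, with that visual step skipped on dedicated servers.
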(event `self.Capsule.OnComponentBeginOverlap`
  (params (OverlappedComponent :type "PrimitiveComponent Object Reference") (OtherActor :type "Actor Object Reference") (OtherComp :type "PrimitiveComponent Object Reference") (OtherBodyIndex :type Integer) (bFromSweep :type Boolean) (SweepResult :type "HitResult Structure (by ref)"))
  (`self.Teleport` OtherActor))

(event `ChangeUsable`
  (if (`KismetSystemLibrary.IsServer`)
    (`|ExecutionSequence`
      (:`then_0`
        (if (not (`KismetSystemLibrary.IsDedicatedServer`))
          (`SceneComponent.SetVisibility` (`self.P_Sparks`) false false :!label _label)
          (`KismetSystemLibrary.RetriggerableDelay` 10.0)
          (`SceneComponent.SetVisibility` (`self.P_Sparks`) true true)))
      (:`then_1`
        (set `self.Usable` false)
        (`KismetSystemLibrary.RetriggerableDelay` 10.0)
        (set `self.Usable` true)))
    (else
      (goto _label))))

(fn `Teleport`
  (params (TelepotedActor :type "Actor Object Reference"))
  (locals (L_duo :type "/Game/Blueprints/Maps/Teleport Object Reference"))
  (bind _duo (`self.Duo`))
  (if (`KismetSystemLibrary.IsServer`)
    (if (`self.Usable`)
      (bind _output_get (set `local.L_duo` (`|GetArrayItem` _duo (`KismetMathLibrary.RandomIntegerInRange` 0 (`KismetArrayLibrary.Array_LastIndex` _duo)))))
      (`self.ChangeUsable` _output_get)
      (`self.ChangeUsable`)
      (`self.K2_SetActorLocation` TelepotedActor (+ (`self.K2_GetActorLocation` _output_get) (- (`self.K2_GetActorLocation` TelepotedActor) (`self.K2_GetActorLocation`))) false true))))

(fn `UserConstructionScript`)